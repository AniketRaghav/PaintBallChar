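; Parent Blueprint for affected objects that apply a color-based effect to the first-person character.
; BeginAffectingObject casts the incoming actor to BP_FirstPersonCharacter, then SetEffect switches on ColorEffect to call the Green, Red, Blue, Yellow or Grey effect function.
; All five effect functions are empty here; Red and Blue hold only unconnected walk-speed and gravity-scale nodes that never run.
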(event Custom|Begin%20Affecting%20Object
  (params (Actor :type BP%20First%20Person%20Character%20Object%20Reference))
  (bind _asbp_first_person_character (Utilities|Casting|CastToBP_FirstPersonCharacter Actor))
  (CallFunction|SetEffect _asbp_first_person_character))

(fn ConstructionScript)

(fn SetEffect
  (params (Character :type Actor%20Object%20Reference))
  (switch Utilities|FlowControl|Switch|SwitchonColorEffect (Variables|Default|GetColorEffect)
    (:NewEnumerator0
      (CallFunction|GreenEffect Character))
    (:NewEnumerator1
      (CallFunction|RedEffect Character))
    (:NewEnumerator2
      (CallFunction|BlueEffect Character))
    (:NewEnumerator3
      (CallFunction|YellowEffect Character))
    (:NewEnumerator4
      (CallFunction|GreyEffect Character))))

(fn GreenEffect
  (params (Character :type Actor%20Object%20Reference)))

(fn RedEffect
  (params (Character :type Actor%20Object%20Reference)))

(fn BlueEffect
  (params (Character :type Actor%20Object%20Reference)))

(fn YellowEffect
  (params (Character :type Actor%20Object%20Reference)))

(fn GreyEffect
  (params (Character :type Actor%20Object%20Reference)))