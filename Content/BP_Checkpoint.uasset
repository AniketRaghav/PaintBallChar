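; Checkpoint actor that sets the player's respawn point when a PaintBallChar overlaps its Box, using the Billboard's world location.
; A Reuse flag lets it fire on every overlap; otherwise it fires once and changes the Cylinder's material.
; When RequiredForFinish, it tags itself "Required" at BeginPlay, and its first collection increments the Finish's CollectedCheckpoints and plays a sound.
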(event OnComponentBeginOverlap(Box)
  (params (OverlappedComponent :type Primitive%20Component%20Object%20Reference) (OtherActor :type Actor%20Object%20Reference) (OtherComp :type Primitive%20Component%20Object%20Reference) (OtherBodyIndex :type Integer) (bFromSweep :type Boolean) (SweepResult :type Hit%20Result%20Structure%20%28by%20ref%29))
  (bind (_aspaint_ball_char _bsuccess) (Utilities|Casting|CastToPaintBallChar OtherActor))
  ;[1 1 1] Collide With Player
  (if _bsuccess
    (if (Variables|Reusable|GetReuse)
      (Development|PrintString "Collided With Player" :!label _label)
      (Variables|/Game/Tech/Character/PaintBallChar.PaintBallChar_C|SetRespawn%20Point _aspaint_ball_char (Transformation|GetWorldLocation (Variables|Default|GetBillboard)))
      (if (Variables|Collection|GetRequiredForFinish)
        (if (not (Variables|Collection|GetCollected))
          (Variables|Collection|SetCollected true)
          (Math|Integer|IncrementInt (Variables|/Game/Tech/Blueprints/ObstacleBlueprints/GeneralObstacles/BP_Finish.BP_Finish_C|GetCollectedCheckpoints (Variables|Collection|GetFinish))
            (:%20%20
              (Audio|PlaySoundatLocation "/Game/Sounds/CheckPoint.CheckPoint" (Transformation|GetActorLocation) "0, 0, 0" 1.0 1.0 0.0 0 0 0 0)))))
      (elif (not (Variables|Reusable|GetUsed))
        (Variables|Reusable|SetUsed true)
        (Rendering|Material|SetMaterial (Variables|Default|GetCylinder) 0 0)
        (goto _label)))))

(event EventBeginPlay
  ;[1 1 1] Setup
  (if (Variables|Reusable|GetReuse)
    (Rendering|Material|SetMaterial (Variables|Default|GetCylinder) 0 0)
    (else
      (Rendering|Material|SetMaterial (Variables|Default|GetCylinder) 0 0)))
  (if (Variables|Collection|GetRequiredForFinish)
    (Variables|Default|SetTags self (Utilities|Array|MakeArray "Required"))))

(fn ConstructionScript)