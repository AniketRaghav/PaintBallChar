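; BP_Finish is a finish-line trigger that ends the game once the player has collected all required checkpoints.
; When a PaintBallChar overlaps its Box, it compares the count of actors tagged "Required" against CollectedCheckpoints.
; On a match it prints "Finished" and quits the game after a short delay; otherwise it prints how many checkpoints are still needed.
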(event OnComponentBeginOverlap(Box)
  (params (OverlappedComponent :type Primitive%20Component%20Object%20Reference) (OtherActor :type Actor%20Object%20Reference) (OtherComp :type Primitive%20Component%20Object%20Reference) (OtherBodyIndex :type Integer) (bFromSweep :type Boolean) (SweepResult :type Hit%20Result%20Structure%20%28by%20ref%29))
  (bind _collectedcheckpoints (Variables|Default|GetCollectedCheckpoints))
  ;[1 1 1] Collides With Player
  (if (.bSuccess (Utilities|Casting|CastToPaintBallChar OtherActor))
    (bind _outactors (Actor|GetAllActorsOfClasswithTag 0 "Required"))
    (if (== (Utilities|Array|Length _outactors) _collectedcheckpoints)
      (Development|PrintString "Finished")
      (Utilities|FlowControl|Delay 0.5)
      (Game|QuitGame 0 "Quit" false)
      (else
        (Development|PrintString (Utilities|String|Append "Need " (Utilities|String|ToString(Integer) (- (Utilities|Array|Length _outactors) _collectedcheckpoints)) " more checkpoints"))))))

(fn ConstructionScript)