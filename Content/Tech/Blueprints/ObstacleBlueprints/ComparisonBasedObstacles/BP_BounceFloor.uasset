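; Paint-activated bounce floor obstacle that launches the PaintBallChar on overlap while it is active.
; When SetColorEnum receives a color matching its own Enum, it turns pink and sets IsSafe, which enables the launch.
; A 10-second timer then clears IsSafe through ResetColor, without restoring the material.
; Random color cycling through RandomizeColor and DecideWhichColor exists, but its looping timer is never run.
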(event OnComponentBeginOverlap(Box)
  (params (OverlappedComponent :type Primitive%20Component%20Object%20Reference) (OtherActor :type Actor%20Object%20Reference) (OtherComp :type Primitive%20Component%20Object%20Reference) (OtherBodyIndex :type Integer) (bFromSweep :type Boolean) (SweepResult :type Hit%20Result%20Structure%20%28by%20ref%29))
  (if (Variables|Default|GetisSafe)
    (bind _aspaint_ball_char (Utilities|Casting|CastToPaintBallChar OtherActor))
    (Character|LaunchCharacter _aspaint_ball_char (Variables|Default|GetLaunch%20Amount) false false)))

(event EventBeginPlay)

(event Collision|EventActorBeginOverlap
  (params (OtherActor :type Actor%20Object%20Reference)))

(event EventTick
  (params (DeltaSeconds :type Float%20%28single-precision%29)))

(event EventSetColorEnum
  (params (ColorState :type E_ColorEffect%20Enum :default "NewEnumerator6"))
  (if (Utilities|Enum|Equal(Enum) ColorState (Variables|Default|GetEnum))
    (Variables|Default|SetisSafe true)
    (CallFunction|SetColorMaterial "/Game/Art/PaintColourInstances/MI_PaintColours_Pink.MI_PaintColours_Pink")
    (Utilities|Time|SetTimerbyFunctionName 0 "ResetColor" 1e+01)
    (else
      (Development|PrintString "Hello"))))

(fn ConstructionScript
  (|CallParentFunction))

(fn RandomizeColor
  (switch int (Math|Random|RandomInteger 5)
    (:0
      (Variables|Default|SetEnum "NewEnumerator0"))
    (:1
      (Variables|Default|SetEnum "NewEnumerator1"))
    (:2
      (Variables|Default|SetEnum "NewEnumerator2"))
    (:3
      (Variables|Default|SetEnum "NewEnumerator3"))
    (:4
      (Variables|Default|SetEnum "NewEnumerator4")))
  (CallFunction|DecideWhichColor))

(fn DecideWhichColor
  (switch Utilities|FlowControl|Switch|SwitchonE_ColorEffect (Variables|Default|GetEnum)
    (:NewEnumerator3
      (LocalVariables|SetMaterial "/Game/UnrealContent/FPWeapon/Materials/FirstPersonProjectileMaterial.FirstPersonProjectileMaterial"))
    (:NewEnumerator1
      (LocalVariables|SetMaterial 0))
    (:NewEnumerator0
      (LocalVariables|SetMaterial 0))
    (:NewEnumerator4
      (LocalVariables|SetMaterial 0))
    (:NewEnumerator2
      (LocalVariables|SetMaterial "/Game/LevelPrototyping/Materials/MI_Solid_Blue.MI_Solid_Blue")))
  (CallFunction|SetColorMaterial (LocalVariables|GetMaterial)))

(fn SetColorMaterial
  (params (Color :type Material%20Interface%20Object%20Reference))
  (Rendering|Material|SetMaterial (Variables|Default|GetCube2) 0 Color))

(fn ResetColor
  (Variables|Default|SetisSafe false))

(fn Destroy)