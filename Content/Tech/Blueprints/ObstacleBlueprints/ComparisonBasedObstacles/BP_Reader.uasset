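; BP_Reader is a color-matching obstacle that switches to a random one of five colors every two seconds.
; A looping timer picks the color enum, then maps it to a material applied to all three cubes.
; SetColorEnum compares an incoming color with the current one to set Cube2's collision.
; A match ignores GameTraceChannel1, while a mismatch blocks the Destructible channel instead, so the branches edit different channels.
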(event EventBeginPlay
  (Utilities|Time|SetTimerbyFunctionName 0 "RandomizeColor" 2.0 true))

(event Collision|EventActorBeginOverlap
  (params (OtherActor :type Actor%20Object%20Reference)))

(event EventTick
  (params (DeltaSeconds :type Float%20%28single-precision%29)))

(event EventSetColorEnum
  (params (ColorState :type E_ColorEffect%20Enum :default "NewEnumerator0"))
  (bind _cube2 (Variables|Default|GetCube2))
  (if (Utilities|Enum|Equal(Enum) ColorState (Variables|Default|GetEnum))
    (Collision|SetCollisionResponsetoChannel _cube2 "ECC_GameTraceChannel1" "ECR_Ignore")
    (else
      (Collision|SetCollisionResponsetoChannel _cube2 "ECC_Destructible" "ECR_Block")))
  (Development|PrintString "Set"))

(fn ConstructionScript
  (|CallParentFunction))

(fn RandomizeColor
  (switch int (Math|Random|RandomInteger 5)
    (:0
      (Variables|Default|SetEnum "NewEnumerator0"))
    (:1
      (Variables|Default|SetEnum "NewEnumerator1"))
    (:2
      (Variables|Default|SetEnum "NewEnumerator2"))
    (:3
      (Variables|Default|SetEnum "NewEnumerator3"))
    (:4
      (Variables|Default|SetEnum "NewEnumerator4")))
  (CallFunction|DecideWhichColor))

(fn DecideWhichColor
  (switch Utilities|FlowControl|Switch|SwitchonE_ColorEffect (Variables|Default|GetEnum)
    (:NewEnumerator0
      (LocalVariables|SetMaterial "/Game/StarterContent/Materials/M_Ground_Grass.M_Ground_Grass"))
    (:NewEnumerator1
      (LocalVariables|SetMaterial "/Game/StarterContent/Materials/M_Wood_Floor_Walnut_Polished.M_Wood_Floor_Walnut_Polished"))
    (:NewEnumerator2
      (LocalVariables|SetMaterial "/Game/LevelPrototyping/Materials/MI_Solid_Blue.MI_Solid_Blue"))
    (:NewEnumerator3
      (LocalVariables|SetMaterial "/Game/UnrealContent/FPWeapon/Materials/FirstPersonProjectileMaterial.FirstPersonProjectileMaterial"))
    (:NewEnumerator4
      (LocalVariables|SetMaterial "/Game/StarterContent/Materials/M_Metal_Chrome.M_Metal_Chrome")))
  (CallFunction|SetColors (LocalVariables|GetMaterial)))

(fn SetColors
  (params (Color :type Material%20Interface%20Object%20Reference))
  (Rendering|Material|SetMaterial (Variables|Default|GetCube) 0 Color)
  (Rendering|Material|SetMaterial (Variables|Default|GetCube1) 0 Color)
  (Rendering|Material|SetMaterial (Variables|Default|GetCube2) 0 Color))