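; Slippery floor obstacle that makes a PaintBallChar slide fast with no ground friction while inside its box, restoring fixed movement values on exit.
; When SetColorEnum receives a color matching the floor's enum, the floor becomes safe and changes material for ten seconds before resetting.
; Color randomization picks one of five colors and applies its material, but its looping timer is disconnected and never runs.
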(event OnComponentBeginOverlap(Box)
  (params (OverlappedComponent :type Primitive%20Component%20Object%20Reference) (OtherActor :type Actor%20Object%20Reference) (OtherComp :type Primitive%20Component%20Object%20Reference) (OtherBodyIndex :type Integer) (bFromSweep :type Boolean) (SweepResult :type Hit%20Result%20Structure%20%28by%20ref%29))
  (if (not (Variables|Default|GetisSafe))
    (bind _aspaint_ball_char (Utilities|Casting|CastToPaintBallChar OtherActor))
    (Variables|/Script/Engine.CharacterMovementComponent|SetGroundFriction (Variables|/Script/Engine.Character|GetCharacterMovement _aspaint_ball_char) 0.0)
    (Variables|/Script/Engine.CharacterMovementComponent|SetBrakingDecelerationWalking (Variables|/Script/Engine.Character|GetCharacterMovement _aspaint_ball_char) -1e+02)
    (Variables|/Script/Engine.CharacterMovementComponent|SetMaxAcceleration (Variables|/Script/Engine.Character|GetCharacterMovement _aspaint_ball_char) 2.048e+05)
    (Variables|/Script/Engine.CharacterMovementComponent|SetMaxWalkSpeed (Variables|/Script/Engine.Character|GetCharacterMovement _aspaint_ball_char) 1.5e+03)))

(event OnComponentEndOverlap(Box)
  (params (OverlappedComponent :type Primitive%20Component%20Object%20Reference) (OtherActor :type Actor%20Object%20Reference) (OtherComp :type Primitive%20Component%20Object%20Reference) (OtherBodyIndex :type Integer))
  (bind _aspaint_ball_char (Utilities|Casting|CastToPaintBallChar OtherActor))
  (Variables|/Script/Engine.CharacterMovementComponent|SetGroundFriction (Variables|/Script/Engine.Character|GetCharacterMovement _aspaint_ball_char) 8.0)
  (Variables|/Script/Engine.CharacterMovementComponent|SetBrakingDecelerationWalking (Variables|/Script/Engine.Character|GetCharacterMovement _aspaint_ball_char) 2048.0)
  (Variables|/Script/Engine.CharacterMovementComponent|SetMaxAcceleration (Variables|/Script/Engine.Character|GetCharacterMovement _aspaint_ball_char) 2048.0)
  (Variables|/Script/Engine.CharacterMovementComponent|SetMaxWalkSpeed (Variables|/Script/Engine.Character|GetCharacterMovement _aspaint_ball_char) 6e+02))

(event EventBeginPlay)

(event Collision|EventActorBeginOverlap
  (params (OtherActor :type Actor%20Object%20Reference)))

(event EventTick
  (params (DeltaSeconds :type Float%20%28single-precision%29)))

(event EventSetColorEnum
  (params (ColorState :type E_ColorEffect%20Enum :default "NewEnumerator6"))
  (if (Utilities|Enum|Equal(Enum) ColorState (Variables|Default|GetEnum))
    (Variables|Default|SetisSafe true)
    (CallFunction|SetColorMaterial "/Game/StarterContent/Props/Materials/M_Shelf.M_Shelf")
    (Utilities|Time|SetTimerbyFunctionName 0 "ResetColor" 1e+01)))

(fn ConstructionScript
  (|CallParentFunction))

(fn RandomizeColor
  (switch int (Math|Random|RandomInteger 5)
    (:0
      (Variables|Default|SetEnum "NewEnumerator0"))
    (:1
      (Variables|Default|SetEnum "NewEnumerator1"))
    (:2
      (Variables|Default|SetEnum "NewEnumerator2"))
    (:3
      (Variables|Default|SetEnum "NewEnumerator3"))
    (:4
      (Variables|Default|SetEnum "NewEnumerator4")))
  (CallFunction|DecideWhichColor))

(fn DecideWhichColor
  (switch Utilities|FlowControl|Switch|SwitchonE_ColorEffect (Variables|Default|GetEnum)
    (:NewEnumerator3
      (LocalVariables|SetMaterial "/Game/UnrealContent/FPWeapon/Materials/FirstPersonProjectileMaterial.FirstPersonProjectileMaterial"))
    (:NewEnumerator1
      (LocalVariables|SetMaterial "/Game/StarterContent/Materials/M_Wood_Floor_Walnut_Polished.M_Wood_Floor_Walnut_Polished"))
    (:NewEnumerator0
      (LocalVariables|SetMaterial "/Game/StarterContent/Materials/M_Ground_Grass.M_Ground_Grass"))
    (:NewEnumerator4
      (LocalVariables|SetMaterial "/Game/StarterContent/Materials/M_Metal_Chrome.M_Metal_Chrome"))
    (:NewEnumerator2
      (LocalVariables|SetMaterial "/Game/LevelPrototyping/Materials/MI_Solid_Blue.MI_Solid_Blue")))
  (CallFunction|SetColorMaterial (LocalVariables|GetMaterial)))

(fn SetColorMaterial
  (params (Color :type Material%20Interface%20Object%20Reference))
  (Rendering|Material|SetMaterial (Variables|Default|GetCube2) 0 Color))

(fn ResetColor
  (Variables|Default|SetisSafe false)
  (CallFunction|SetColorMaterial "/Game/UnrealContent/FPWeapon/Materials/BaseMaterial.BaseMaterial"))