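; Color-driven switch obstacle that reveals a bridge when its color matches that of a linked BridgeSwitch.
; It extends the parent's Set Color Material by applying the material to its mesh and then running Compare.
; On a match, Compare passes the color to the Bridge, unhides its mesh and sets mesh collision to block and box collision to overlap.
; Compare has no mismatch branch, so it never hides the bridge again.
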(event EventBeginPlay
  (|CallParentFunction) ; This node is disabled and will not be called.\nDrag off pins to build functionality.
)

(event Collision|EventActorBeginOverlap
  (params (OtherActor :type Actor%20Object%20Reference))
  (|CallParentFunction OtherActor) ; This node is disabled and will not be called.\nDrag off pins to build functionality.
)

(event EventTick
  (params (DeltaSeconds :type Float%20%28single-precision%29))
  (|CallParentFunction DeltaSeconds) ; This node is disabled and will not be called.\nDrag off pins to build functionality.
)

(fn ConstructionScript
  (|CallParentFunction))

(fn SetColorMaterial
  (params (ColortoSet :type Material%20Interface%20Object%20Reference))
  (|CallParentFunction ColortoSet)
  (Rendering|Material|SetMaterial (Variables|Default|GetStaticMesh) 0 ColortoSet)
  (CallFunction|Compare ColortoSet))

(fn Compare
  (params (MaterialtoSet :type Material%20Interface%20Object%20Reference))
  (bind _color_enum (Variables|Default|GetColor%20Enum))
  (bind _bridge (Variables|Default|GetBridge))
  (bind _staticmesh (Variables|/Game/Tech/Blueprints/ObstacleBlueprints/SwitchControlledObjects/AffectedFloors/AffectedFloor.AffectedFloor_C|GetStaticMesh _bridge))
  (if (Utilities|Enum|Equal(Enum) (Variables|/Game/Tech/Blueprints/ObstacleBlueprints/DirectlyControlled/DirectObjParent.DirectObjParent_C|GetColor%20Enum (Variables|Default|GetBridgeSwitch)) _color_enum)
    (Variables|/Game/Tech/Blueprints/ObstacleBlueprints/SwitchControlledObjects/AffectedFloors/AffectedOBJParent.AffectedOBJParent_C|SetColorEffect _bridge _color_enum)
    (CallFunction|ColortoSet)
    (Development|SetHiddeninGame _staticmesh false false)
    (Collision|SetCollisionResponsetoAllChannels _staticmesh "ECR_Block")
    (Collision|SetCollisionResponsetoAllChannels (Variables|/Game/Tech/Blueprints/ObstacleBlueprints/SwitchControlledObjects/AffectedFloors/AffectedFloor.AffectedFloor_C|GetBox _bridge) "ECR_Overlap")))