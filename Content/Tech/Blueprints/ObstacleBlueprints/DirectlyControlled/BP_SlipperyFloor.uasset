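; BP_SlipperyFloor is a slippery floor obstacle whose walkability responds to color state changes.
; Its SetColor event sets IsWalkable to true for one specific color state and never clears it here.
; Set Color Material is an empty stub, the construction script only calls the parent, and BeginPlay, overlap and Tick are disabled.
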(event Custom|SetColor_1
  (params (ColorState :type E_ColorEffect%20Enum :default "NewEnumerator0"))
  (if (Utilities|Enum|Equal(Enum) ColorState "NewEnumerator3")
    (Variables|Default|SetIsWalkable true)))

(event EventBeginPlay
  (|CallParentFunction) ; This node is disabled and will not be called.\nDrag off pins to build functionality.
)

(event Collision|EventActorBeginOverlap
  (params (OtherActor :type Actor%20Object%20Reference))
  (|CallParentFunction OtherActor) ; This node is disabled and will not be called.\nDrag off pins to build functionality.
)

(event EventTick
  (params (DeltaSeconds :type Float%20%28single-precision%29))
  (|CallParentFunction DeltaSeconds) ; This node is disabled and will not be called.\nDrag off pins to build functionality.
)

(fn ConstructionScript
  (|CallParentFunction))

(fn SetColorMaterial
  (params (ColortoSet :type Material%20Interface%20Object%20Reference)))