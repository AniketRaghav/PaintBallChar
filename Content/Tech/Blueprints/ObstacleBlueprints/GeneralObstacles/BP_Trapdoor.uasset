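; BP_Trapdoor is a two-door trapdoor obstacle that swings open shortly after a PaintBallChar overlaps its detection volume.
; Tick drives Move, which counter-rotates the hinges through a remaining-angle counter, snaps them when closed, and sets a timer to Close after opening.
; PaintSphere hits on either door toggle IsGlued by color effect: one freezes movement, another releases it and resumes any unfinished swing.
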(event OnComponentBeginOverlap(PlayerDetection)
  (params (OverlappedComponent :type Primitive%20Component%20Object%20Reference) (OtherActor :type Actor%20Object%20Reference) (OtherComp :type Primitive%20Component%20Object%20Reference) (OtherBodyIndex :type Integer) (bFromSweep :type Boolean) (SweepResult :type Hit%20Result%20Structure%20%28by%20ref%29))
  (Utilities|Casting|CastToPaintBallChar OtherActor)
  (if (not (Variables|Default|GetisGlued?))
    (Utilities|FlowControl|Delay (Variables|Default|GetDelay))
    (CallFunction|Open)))

(event OnComponentHit(LeftDoor)
  (params (HitComponent :type Primitive%20Component%20Object%20Reference) (OtherActor :type Actor%20Object%20Reference) (OtherComp :type Primitive%20Component%20Object%20Reference) (NormalImpulse :type Vector :default "0, 0, 0") (Hit :type Hit%20Result%20Structure%20%28by%20ref%29))
  (bind _aspaint_sphere (Utilities|Casting|CastToPaintSphere OtherActor))
  (if (Utilities|Enum|Equal(Enum) (Variables|/Game/Tech/Blueprints/PaintSpheresandEffects/PaintSphere.PaintSphere_C|GetColor%20Effect _aspaint_sphere) "NewEnumerator0")
    (if (not (Variables|Default|GetisGlued?))
      (Variables|Default|SetisGlued? true)
      (Variables|Default|SetisOpening? false))
    (elif (Utilities|Enum|Equal(Enum) (Variables|/Game/Tech/Blueprints/PaintSpheresandEffects/PaintSphere.PaintSphere_C|GetColor%20Effect _aspaint_sphere) "NewEnumerator6")
      (if (Variables|Default|GetisGlued?)
        (Variables|Default|SetisGlued? false)
        (if (> (Variables|Default|GetDistanceToRotate) 0.0)
          (Variables|Default|SetisOpening? true))))))

(event OnComponentHit(RightDoor)
  (params (HitComponent :type Primitive%20Component%20Object%20Reference) (OtherActor :type Actor%20Object%20Reference) (OtherComp :type Primitive%20Component%20Object%20Reference) (NormalImpulse :type Vector :default "0, 0, 0") (Hit :type Hit%20Result%20Structure%20%28by%20ref%29))
  (bind _aspaint_sphere (Utilities|Casting|CastToPaintSphere OtherActor))
  (if (Utilities|Enum|Equal(Enum) (Variables|/Game/Tech/Blueprints/PaintSpheresandEffects/PaintSphere.PaintSphere_C|GetColor%20Effect _aspaint_sphere) "NewEnumerator0")
    (if (not (Variables|Default|GetisGlued?))
      (Variables|Default|SetisGlued? true)
      (Variables|Default|SetisOpening? false))
    (elif (Utilities|Enum|Equal(Enum) (Variables|/Game/Tech/Blueprints/PaintSpheresandEffects/PaintSphere.PaintSphere_C|GetColor%20Effect _aspaint_sphere) "NewEnumerator6")
      (if (Variables|Default|GetisGlued?)
        (Variables|Default|SetisGlued? false)
        (if (> (Variables|Default|GetDistanceToRotate) 0.0)
          (Variables|Default|SetisOpening? true))))))

(event EventTick
  (params (DeltaSeconds :type Float%20%28single-precision%29))
  (CallFunction|Move DeltaSeconds))

(fn ConstructionScript)

(fn Open
  (if (not (Variables|Default|GetisOpen?))
    (if (not (Variables|Default|GetisOpening?))
      (Variables|Default|SetDirection 1.0)
      (if (== (Variables|Default|GetDistanceToRotate) 0.0)
        (Variables|Default|SetDistanceToRotate 9e+01))
      (Variables|Default|SetisOpening? true))))

(fn Close
  (if (not (Variables|Default|GetisGlued?))
    (Variables|Default|SetDirection -1.0)
    (if (== (Variables|Default|GetDistanceToRotate) 0.0)
      (Variables|Default|SetDistanceToRotate 9e+01))
    (Variables|Default|SetisOpening? true)))

(fn Move
  (params (DeltaTime :type Float%20%28double-precision%29))
  (bind _returnvalue (* DeltaTime 1e+02))
  (bind _righthinge (Variables|Default|GetRightHinge))
  (bind _lefthinge (Variables|Default|GetLeftHinge))
  (bind _relativerotation (Variables|/Script/Engine.SceneComponent|GetRelativeRotation _righthinge))
  (bind _relativerotation_2 (Variables|/Script/Engine.SceneComponent|GetRelativeRotation _lefthinge))
  (bind (_roll _pitch _yaw) (Math|Rotator|BreakRotator _relativerotation))
  (bind (_roll_2 _pitch_2 _yaw_2) (Math|Rotator|BreakRotator _relativerotation_2))
  (if (Variables|Default|GetisOpening?)
    (Transformation|AddLocalRotation (Variables|Default|GetRightHinge) (Math|Rotator|MakeRotator 0.0 0.0 (* _returnvalue (Variables|Default|GetDirection))) false false)
    (Transformation|AddLocalRotation (Variables|Default|GetLeftHinge) (Math|Rotator|MakeRotator 0.0 0.0 (* _returnvalue -1.0 (Variables|Default|GetDirection))) false false)
    (bind _output_get (Variables|Default|SetDistanceToRotate (- (Variables|Default|GetDistanceToRotate) _returnvalue)))
    (if (<= _output_get 0.0)
      (Variables|Default|SetisOpening? false)
      (if (Variables|Default|GetisOpen?)
        (Variables|Default|SetisOpen? false)
        (Variables|Default|SetDistanceToRotate 0.0)
        (Transformation|SetRelativeRotation _lefthinge (Math|Rotator|MakeRotator _roll_2 -9e+01 _yaw_2) false false)
        (Transformation|SetRelativeRotation _righthinge (Math|Rotator|MakeRotator _roll -9e+01 _yaw) false false)
        (else
          (Variables|Default|SetisOpen? true)
          (Variables|Default|SetDistanceToRotate 0.0)
          (Utilities|Time|SetTimerbyFunctionName 0 "Close" (Variables|Default|GetOpenDuration)))))))