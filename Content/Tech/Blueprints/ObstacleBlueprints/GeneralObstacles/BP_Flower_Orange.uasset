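; BP_Flower_Orange is an obstacle Blueprint, named as the orange flower variant, that changes its look based on the paintball character's color.
; Its SetMaterial override calls the parent, then compares the character's ColorEffect with the obstacle's Color.
; A match applies the inactive material to Cube1 and Cube2, while any other color applies the active one.
; BeginPlay, overlap and Tick events are disabled placeholders, and construction only calls the parent.
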(event EventBeginPlay
  (|CallParentFunction) ; This node is disabled and will not be called.\nDrag off pins to build functionality.
)

(event Collision|EventActorBeginOverlap
  (params (OtherActor :type Actor%20Object%20Reference)))

(event EventTick
  (params (DeltaSeconds :type Float%20%28single-precision%29)))

(fn ConstructionScript
  (|CallParentFunction))

(fn SetMaterial
  (params (PaintBallCharacter :type Paint%20Ball%20Char%20Object%20Reference))
  (|CallParentFunction 0)
  (if (Utilities|Enum|Equal(Enum) (Variables|/Game/Tech/FirstPerson/Blueprints/BP_FirstPersonCharacter.BP_FirstPersonCharacter_C|GetColorEffect PaintBallCharacter) (Variables|Default|GetColor))
    (Rendering|Material|SetMaterial (Variables|Default|GetCube2) 0 (Variables|Default|GetInActiveMaterial))
    (else
      (Rendering|Material|SetMaterial (Variables|Default|GetCube1) 0 (Variables|Default|GetActiveMaterial)))))