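; Push trap obstacle whose cube slides out by a set distance and back when its main collision cube is hit.
; It either toggles per trigger or auto-retracts on a timer, with Tick moving the cube at a rate from Distance and Time.
; A paint sphere of one color effect doubles travel time until movement stops.
; Size and arrow length are applied at BeginPlay; the damage box overlap has no effect yet.
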(event OnComponentBeginOverlap(DamageBox)
  (params (OverlappedComponent :type Primitive%20Component%20Object%20Reference) (OtherActor :type Actor%20Object%20Reference) (OtherComp :type Primitive%20Component%20Object%20Reference) (OtherBodyIndex :type Integer) (bFromSweep :type Boolean) (SweepResult :type Hit%20Result%20Structure%20%28by%20ref%29))
  (Utilities|Casting|CastToPaintBallChar OtherActor))

(event OnComponentHit(MainCollisionCube)
  (params (HitComponent :type Primitive%20Component%20Object%20Reference) (OtherActor :type Actor%20Object%20Reference) (OtherComp :type Primitive%20Component%20Object%20Reference) (NormalImpulse :type Vector :default "0, 0, 0") (Hit :type Hit%20Result%20Structure%20%28by%20ref%29))
  ;[0.05208 0.05208 0.05208] Replace exec with triggers to activate trap.
  (CallFunction|TriggerTrap)
  (bind _aspaint_sphere (Utilities|Casting|CastToPaintSphere OtherActor))
  (if (Utilities|Enum|Equal(Enum) (Variables|/Game/Tech/Blueprints/PaintSpheresandEffects/PaintSphere.PaintSphere_C|GetColor%20Effect _aspaint_sphere) "NewEnumerator4")
    (if (not (Variables|Default|GetisSlowed?))
      (CallFunction|ToggleSlow true))))

(event Custom|TriggerTrap
  ;[0.05729 0.05729 0.05729] If toggle, stays open until triggered again. otherwise sets a timer to close automatically.
  (if (Variables|Default|GetisToggle?)
    (CallFunction|Extend (not (Variables|Default|GetisOpen?)))
    (elif (not (Variables|Default|GetisOpen?))
      (CallFunction|Extend true)
      (Utilities|Time|SetTimerbyFunctionName 0 "Retract" (+ (Variables|Default|GetTime) 2.0)))))

(event EventBeginPlay
  (bind _size (Variables|Default|GetSize))
  ;[0.06771 0.06771 0.06771] Sets size when runtime starts so designers can change size on the fly.
  (Transformation|SetRelativeScale3D (Variables|Default|GetCube) (Math|Vector|MakeVector _size _size 0.5))
  (Transformation|SetRelativeScale3D (Variables|Default|GetArrow) (Math|Vector|MakeVector 1.0 1.0 (Variables|Default|GetDistance)))
  (Variables|Default|SetBaseTime (Variables|Default|GetTime)))

(event EventTick
  (params (DeltaSeconds :type Float%20%28single-precision%29))
  ;[0.05729 0.05729 0.05729] Attempts to move every tick while isMoving? is true.
  (CallFunction|Movement))

(fn ConstructionScript)

(fn Extend
  (params (Open :type Boolean))
  ;[0.0625 0.0625 0.0625] True extends, false retracts
  (if (not (Variables|Default|GetisMoving?))
    (Variables|Default|SetisMoving? true)
    (Variables|Default|SetDistanceToTravel (* (Variables|Default|GetDistance) 5e+01))
    (Variables|Default|SetOpening Open)))

(fn StopMoving
  (Variables|Default|SetisMoving? false)
  (Variables|Default|SetisOpen? (Variables|Default|GetOpening))
  (CallFunction|ToggleSlow false))

(fn Movement
  (bind _returnvalue (Utilities|Time|GetWorldDeltaSeconds))
  (bind _returnvalue_2 (Utilities|Time|GetWorldDeltaSeconds))
  (bind _distance (Variables|Default|GetDistance))
  (bind _time (Variables|Default|GetTime))
  (bind _distance_2 (Variables|Default|GetDistance))
  (bind _time_2 (Variables|Default|GetTime))
  (bind _returnvalue_3 (* _distance_2 5e+01))
  (bind _returnvalue_4 (* _distance 5e+01))
  (bind _returnvalue_5 (/ _returnvalue_4 _time))
  (bind _returnvalue_6 (/ _returnvalue_3 _time_2))
  (bind _returnvalue_7 (* _returnvalue_5 _returnvalue))
  (bind _returnvalue_8 (* _returnvalue_6 _returnvalue_2))
  ;[0.04167 0.04167 0.04167] Movement. If Opening is true, moves foward, otherwise it moves back.
  (if (Variables|Default|GetisMoving?)
    (if (Variables|Default|GetOpening)
      (Transformation|AddRelativeLocation (Variables|Default|GetCube) (Math|Vector|MakeVector 0.0 0.0 _returnvalue_8) false false)
      (bind _output_get (Variables|Default|SetDistanceToTravel (- (Variables|Default|GetDistanceToTravel) _returnvalue_8)))
      (if (<= _output_get 0.0)
        (CallFunction|StopMoving :!label _label))
      (else
        (Transformation|AddRelativeLocation (Variables|Default|GetCube) (Math|Vector|MakeVector 0.0 0.0 (* _returnvalue_7 -1.0)) false false)
        (bind _output_get_2 (Variables|Default|SetDistanceToTravel (- (Variables|Default|GetDistanceToTravel) _returnvalue_7)))
        (if (<= _output_get_2 0.0)
          (goto _label))))))

(fn Retract
  (CallFunction|Extend false))

(fn ToggleSlow
  (params (Value :type Boolean))
  (bind _output_get (Variables|Default|SetisSlowed? Value))
  (if _output_get
    (Variables|Default|SetTime (* (Variables|Default|GetBaseTime) 2.0))
    (else
      (Variables|Default|SetTime (Variables|Default|GetBaseTime)))))