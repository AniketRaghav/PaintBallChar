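; BP_PaintFlower is a colour-coded paint obstacle with text labels for its colour and ammo count.
; The construction script uses the Color enum to set the cube's material, the label text and both text colours.
; SetAmmoText writes the rounded AmmoCount but is not called here, and SetMesh assigns no mesh for any colour.
; The Purple value uses a pink material and a brown "Brown" label.
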(fn ConstructionScript
  (CallFunction|WhichColortoSet))

(fn SetAmmoText
  (Rendering|Components|TextRender|SetText (Variables|Default|GetCountText) (Utilities|Text|ToText(Integer) (Math|Float|Round (Variables|Default|GetAmmoCount)))))

(fn WhichColortoSet
  (bind _colourtext (Variables|Default|GetColourText))
  (bind _colourtext_2 (Variables|Default|GetColourText))
  (switch Utilities|FlowControl|Switch|SwitchonE_ColorEffect (Variables|Default|GetColor)
    (:NewEnumerator3
      (LocalVariables|SetMaterialInterface "/Game/Art/PaintColourInstances/MI_PaintColours_Yellow.MI_PaintColours_Yellow"))
    (:NewEnumerator1
      (LocalVariables|SetMaterialInterface "/Game/Art/PaintColourInstances/MI_PaintColours_Pink.MI_PaintColours_Pink"))
    (:NewEnumerator0
      (LocalVariables|SetMaterialInterface "/Game/Art/PaintColourInstances/MI_PaintColours_Green.MI_PaintColours_Green"))
    (:NewEnumerator5
      (LocalVariables|SetMaterialInterface "/Game/Art/PaintColourInstances/MI_PaintColours_Orange.MI_PaintColours_Orange"))
    (:NewEnumerator4
      (LocalVariables|SetMaterialInterface "/Game/Art/PaintColourInstances/MI_PaintColours_Grey.MI_PaintColours_Grey"))
    (:NewEnumerator2
      (LocalVariables|SetMaterialInterface "/Game/Art/PaintColourInstances/MI_PaintColours_Blue_001.MI_PaintColours_Blue_001")))
  (CallFunction|SetMaterial (LocalVariables|GetMaterialInterface))
  (switch Utilities|FlowControl|Switch|SwitchonE_ColorEffect (Variables|Default|GetColor)
    (:NewEnumerator3
      (Rendering|Components|TextRender|SetText _colourtext_2 (Utilities|Text|MakeLiteralText "Yellow"))
      (Rendering|Components|TextRender|SetTextRenderColor _colourtext (Math|Color|MakeColor 0 255 255 1)))
    (:NewEnumerator1
      (Rendering|Components|TextRender|SetText _colourtext_2 (Utilities|Text|MakeLiteralText "Brown"))
      (Rendering|Components|TextRender|SetTextRenderColor _colourtext (Math|Color|MakeColor 17 71 155 1)))
    (:NewEnumerator0
      (Rendering|Components|TextRender|SetText _colourtext_2 (Utilities|Text|MakeLiteralText "Green"))
      (Rendering|Components|TextRender|SetTextRenderColor _colourtext (Math|Color|MakeColor 0 255 0 1)))
    (:NewEnumerator5
      (Rendering|Components|TextRender|SetText _colourtext_2 (Utilities|Text|MakeLiteralText "Orange"))
      (Rendering|Components|TextRender|SetTextRenderColor _colourtext (Math|Color|MakeColor 0 112 255 1)))
    (:NewEnumerator4
      (Rendering|Components|TextRender|SetText _colourtext_2 (Utilities|Text|MakeLiteralText "Grey"))
      (Rendering|Components|TextRender|SetTextRenderColor _colourtext (Math|Color|MakeColor 112 112 122 1)))
    (:NewEnumerator2
      (Rendering|Components|TextRender|SetText _colourtext_2 (Utilities|Text|MakeLiteralText "Blue"))
      (Rendering|Components|TextRender|SetTextRenderColor _colourtext (Math|Color|MakeColor 255 0 0 1))))
  (Rendering|Components|TextRender|SetTextRenderColor (Variables|Default|GetCountText) (Variables|/Script/Engine.TextRenderComponent|GetTextRenderColor (Variables|Default|GetColourText))))

(fn SetMaterial
  (params (MaterialInterface :type Material%20Interface%20Object%20Reference))
  (Rendering|Material|SetMaterial (Variables|Default|GetCube) 0 MaterialInterface))

(fn SetMesh
  (switch Utilities|FlowControl|Switch|SwitchonE_ColorEffect (Variables|Default|GetColor)
    (:NewEnumerator3
      (Variables|Default|SetMesh 0))
    (:NewEnumerator1
      (Variables|Default|SetMesh 0))
    (:NewEnumerator0
      (Variables|Default|SetMesh 0))
    (:NewEnumerator5
      (Variables|Default|SetMesh 0))
    (:NewEnumerator4
      (Variables|Default|SetMesh 0))
    (:NewEnumerator2
      (Variables|Default|SetMesh 0))))