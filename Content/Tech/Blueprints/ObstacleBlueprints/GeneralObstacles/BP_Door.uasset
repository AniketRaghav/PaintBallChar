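; BP_Door is an obstacle door that opens once by jumping to an offset position when its Open event fires.
; Open records the Cube's world location, adds TargetLocation and moves the whole actor there in a single swept move.
; An IsOpen flag blocks repeat opens, and the file has no close logic.
; A Timeline, a vector lerp and a Cube-only move remain disconnected, so the motion is not animated.
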(event Custom|Open
  (if (not (Variables|Default|GetisOpen))
    (Variables|Default|SetStartLocation (Transformation|GetWorldLocation (Variables|Default|GetCube)))
    (Transformation|SetActorLocation (+ (Variables|Default|GetStartLocation) (Variables|Default|GetTargetLocation)) true false)
    (Variables|Default|SetisOpen true)))

(fn ConstructionScript)