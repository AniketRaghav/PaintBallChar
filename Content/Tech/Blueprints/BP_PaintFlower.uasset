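; BP_PaintFlower is an actor with a paint Color and an ammo count, shown through two text components.
; On BeginPlay, SetColor switches on the Color enum to set the colour name and tint, then copies that tint to the count text, as a temporary way to distinguish colours.
; SetAmmoText writes the rounded AmmoCount to the count text, but nothing in this Blueprint calls it.
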(event Custom|SetColor
  (bind _colourtext (Variables|Default|GetColourText))
  (bind _colourtext_2 (Variables|Default|GetColourText))
  ;[0.07292 0.07292 0.07292] Temporary way to distinguish colour
  (switch Utilities|FlowControl|Switch|SwitchonE_ColorEffect (Variables|Default|GetColor)
    (:NewEnumerator0
      (Rendering|Components|TextRender|SetText _colourtext_2 (Utilities|Text|MakeLiteralText "Green"))
      (Rendering|Components|TextRender|SetTextRenderColor _colourtext (Math|Color|MakeColor 0 255 0 1)))
    (:NewEnumerator1
      (Rendering|Components|TextRender|SetText _colourtext_2 (Utilities|Text|MakeLiteralText "Brown"))
      (Rendering|Components|TextRender|SetTextRenderColor _colourtext (Math|Color|MakeColor 17 71 155 1)))
    (:NewEnumerator2
      (Rendering|Components|TextRender|SetText _colourtext_2 (Utilities|Text|MakeLiteralText "Blue"))
      (Rendering|Components|TextRender|SetTextRenderColor _colourtext (Math|Color|MakeColor 255 0 0 1)))
    (:NewEnumerator3
      (Rendering|Components|TextRender|SetText _colourtext_2 (Utilities|Text|MakeLiteralText "Yellow"))
      (Rendering|Components|TextRender|SetTextRenderColor _colourtext (Math|Color|MakeColor 0 255 255 1)))
    (:NewEnumerator4
      (Rendering|Components|TextRender|SetText _colourtext_2 (Utilities|Text|MakeLiteralText "Grey"))
      (Rendering|Components|TextRender|SetTextRenderColor _colourtext (Math|Color|MakeColor 112 112 122 1))))
  (Rendering|Components|TextRender|SetTextRenderColor (Variables|Default|GetCountText) (Variables|/Script/Engine.TextRenderComponent|GetTextRenderColor (Variables|Default|GetColourText))))

(event EventBeginPlay
  ;[0.07292 0.07292 0.07292] Temporary way to distinguish colour
  (CallFunction|SetColor))

(fn ConstructionScript)

(fn SetAmmoText
  (Rendering|Components|TextRender|SetText (Variables|Default|GetCountText) (Utilities|Text|ToText(Integer) (Math|Float|Round (Variables|Default|GetAmmoCount)))))