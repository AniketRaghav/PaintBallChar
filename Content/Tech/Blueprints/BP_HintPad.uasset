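; BP_HintPad is a trigger pad that shows a text hint when the PaintBallChar steps into its box.
; On overlap, if enabled, it creates a W_HintText widget, fills it with DisplayedText, shows the mouse cursor and blocks move and look input.
; Any end overlap on the box clears Enabled, disabling further hints; nothing here removes the widget or restores input.
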(event OnComponentBeginOverlap(Box)
  (params (OverlappedComponent :type Primitive%20Component%20Object%20Reference) (OtherActor :type Actor%20Object%20Reference) (OtherComp :type Primitive%20Component%20Object%20Reference) (OtherBodyIndex :type Integer) (bFromSweep :type Boolean) (SweepResult :type Hit%20Result%20Structure%20%28by%20ref%29))
  (bind _returnvalue (Game|GetPlayerController 0))
  (if (Variables|Default|GetEnabled)
    (Utilities|Casting|CastToPaintBallChar OtherActor)
    (bind _returnvalue_2 (UserInterface|CreateWidget "/Game/Tech/Menus/W_HintText.W_HintText_C" (Game|GetPlayerController 0)))
    (bind _output_get (Variables|Default|SetCurrentTextWidget _returnvalue_2))
    (UserInterface|Viewport|AddtoViewport _output_get 0)
    (Variables|/Script/UMG.TextBlock|SetText (Variables|/Game/Tech/Menus/W_HintText.W_HintText_C|GetTxt_Hint _output_get) (Variables|Default|GetDisplayedText))
    (Variables|/Script/Engine.PlayerController|SetbShowMouseCursor _returnvalue true)
    (Input|SetIgnoreMoveInput _returnvalue true)
    (Input|SetIgnoreLookInput _returnvalue true)))

(event OnComponentEndOverlap(Box)
  (params (OverlappedComponent :type Primitive%20Component%20Object%20Reference) (OtherActor :type Actor%20Object%20Reference) (OtherComp :type Primitive%20Component%20Object%20Reference) (OtherBodyIndex :type Integer))
  (Variables|Default|SetEnabled false))

(fn ConstructionScript)