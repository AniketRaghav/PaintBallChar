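; BP_HealingCircle is a temporary healing zone actor that restores health to a PaintBallChar standing inside its capsule, then destroys itself ten seconds after spawning.
; Capsule overlap stores the entering character, sets an inside flag and starts a looping timer calling HealPlayer every few seconds.
; HealPlayer adds uncapped health and prints a debug string while the flag is set; exit clears only the flag, and only one character is tracked.
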(event OnComponentBeginOverlap(Capsule)
  (params (OverlappedComponent :type Primitive%20Component%20Object%20Reference) (OtherActor :type Actor%20Object%20Reference) (OtherComp :type Primitive%20Component%20Object%20Reference) (OtherBodyIndex :type Integer) (bFromSweep :type Boolean) (SweepResult :type Hit%20Result%20Structure%20%28by%20ref%29))
  (bind _aspaint_ball_char (Utilities|Casting|CastToPaintBallChar OtherActor))
  (Variables|Default|SetAs%20Paint%20Ball%20Char _aspaint_ball_char)
  (Variables|Default|SetisCharacterInside true)
  (Utilities|Time|SetTimerbyFunctionName 0 "HealPlayer" 3.0 true))

(event OnComponentEndOverlap(Capsule)
  (params (OverlappedComponent :type Primitive%20Component%20Object%20Reference) (OtherActor :type Actor%20Object%20Reference) (OtherComp :type Primitive%20Component%20Object%20Reference) (OtherBodyIndex :type Integer))
  (Utilities|Casting|CastToPaintBallChar OtherActor)
  (Variables|Default|SetisCharacterInside false))

(event Collision|EventActorBeginOverlap
  (params (OtherActor :type Actor%20Object%20Reference)))

(event EventTick
  (params (DeltaSeconds :type Float%20%28single-precision%29)))

(event EventBeginPlay
  (Utilities|Time|SetTimerbyFunctionName 0 "Self-Destruct" 1e+01))

(fn ConstructionScript)

(fn HealPlayer
  (bind _as_paint_ball_char (Variables|Default|GetAs%20Paint%20Ball%20Char))
  (if (Variables|Default|GetisCharacterInside)
    (Variables|/Game/Tech/Character/PaintBallChar.PaintBallChar_C|SetHealth _as_paint_ball_char (+ (Variables|/Game/Tech/Character/PaintBallChar.PaintBallChar_C|GetHealth _as_paint_ball_char) 2e+01))
    (Development|PrintString "Hello")))

(fn Self-Destruct
  (Actor|DestroyActor))