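; Prototype manager that randomizes the color effect of objects linked to its receivers.
; Two seconds after BeginPlay, it loops over every entry in the Reciever array and each object in that entry's AffectedObjectstoSet.
; Each object gets its own random pick from five color enum values in ColorEffect, then ColortoSet is called on it.
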(event EventBeginPlay
  (Utilities|FlowControl|Delay 2.0)
  (CallFunction|SetRecievers))

(event Collision|EventActorBeginOverlap
  (params (OtherActor :type Actor%20Object%20Reference)))

(event EventTick
  (params (DeltaSeconds :type Float%20%28single-precision%29)))

(fn ConstructionScript)

(fn SetRecievers
  (for _array_element (Variables|Default|GetReciever)
    (for _array_element_2 (Variables|/Game/Tech/Blueprints/PrototypingBlueprints/Reciever.Reciever_C|GetAffectedObjectstoSet _array_element)
      (bind _newparam (CallFunction|RandomizeEnum))
      (Variables|/Game/Tech/Blueprints/PrototypingBlueprints/SwitchControlledObjects/AffectedFloors/AffectedOBJParent.AffectedOBJParent_C|SetColorEffect _array_element_2 _newparam)
      (Default|ColortoSet _array_element_2))))

(fn RandomizeEnum
  (switch int (Math|Random|RandomInteger 5)
    (:0
      (LocalVariables|SetColor "NewEnumerator0"))
    (:1
      (LocalVariables|SetColor "NewEnumerator1"))
    (:2
      (LocalVariables|SetColor "NewEnumerator2"))
    (:3
      (LocalVariables|SetColor "NewEnumerator3"))
    (:4
      (LocalVariables|SetColor "NewEnumerator4")))
  (return (LocalVariables|GetColor)))