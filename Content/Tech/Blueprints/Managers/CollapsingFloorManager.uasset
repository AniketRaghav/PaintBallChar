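; Manager actor that handles removing and respawning a collapsing floor.
; Its Destroy event destroys the referenced CollapsingFloor, waits a few seconds, spawns a new BPCollapsingFloor at the manager's own transform and plays a landing sound there.
; DestroyTesting repeats the sequence without the sound.
; Neither event stores the spawned floor back into the CollapsingFloor reference.
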(event Custom|Destroy
  (Actor|DestroyActor (Variables|Default|GetCollapsingFloor))
  (Utilities|FlowControl|Delay 3.0)
  (Game|SpawnActorfromClass "/Game/Tech/Blueprints/ObstacleBlueprints/ComparisonBasedObstacles/BPCollapsingFloor.BPCollapsingFloor_C" (Transformation|GetActorTransform) "Undefined" "MultiplyWithRoot" 0 0)
  (Audio|PlaySoundatLocation "/Game/Sounds/Jump-Landing.Jump-Landing" (Transformation|GetActorLocation) "0, 0, 0" 1.0 1.0 0.0 0 0 0 0))

(event Custom|DestroyTesting
  (Actor|DestroyActor (Variables|Default|GetCollapsingFloor))
  (Utilities|FlowControl|Delay 3.0)
  (Game|SpawnActorfromClass "/Game/Tech/Blueprints/ObstacleBlueprints/ComparisonBasedObstacles/BPCollapsingFloor.BPCollapsingFloor_C" (Transformation|GetActorTransform) "Undefined" "MultiplyWithRoot" 0 0))

(fn ConstructionScript)